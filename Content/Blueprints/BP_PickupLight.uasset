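; BP_PickupLight is a torch pickup that snaps to the TouchSocket on the player character's mesh on overlap and disables its collision.
; Its Light and IncreaseIntensity events each pause the game and open a UI-only widget, WB_Choice or WB_Welcome.
; Bound widget callbacks switch on the SpotLight or, on a correct answer, widen its cone, then hide the cursor.
; Disconnected leftover nodes, including a held-item search, never run.
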(event OnComponentBeginOverlap(Sphere)
  (params (OverlappedComponent :type Primitive%20Component%20Object%20Reference) (OtherActor :type Actor%20Object%20Reference) (OtherComp :type Primitive%20Component%20Object%20Reference) (OtherBodyIndex :type Integer) (bFromSweep :type Boolean) (SweepResult :type Hit%20Result%20Structure%20%28by%20ref%29))
  ;[1 1 1] get picked by player
  (bind _asbp_third_person_character (Utilities|Casting|CastToBP_ThirdPersonCharacter OtherActor))
  (Transformation|AttachComponentToComponent (Variables|/Script/Engine.Character|GetMesh _asbp_third_person_character) "TouchSocket" "SnapToTarget" "SnapToTarget" "SnapToTarget" true)
  ;;[1 1 1] Disable collision on Touchlight BP
  (Collision|SetCollisionEnabled (Variables|Default|GetTorchLight) "NoCollision"))

(event Custom|Light
  (bind _returnvalue (Game|GetPlayerController 0))
  ;[1 1 1] Switch on the light
  (bind _returnvalue_2 (UserInterface|CreateWidget "/Game/UI/UI_David/WB_Choice.WB_Choice_C"))
  (UserInterface|Viewport|AddtoViewport _returnvalue_2 0)
  (Game|SetGamePaused true)
  (Input|SetInputModeUIOnly _returnvalue _returnvalue_2 "DoNotLock" false)
  (Variables|/Script/Engine.PlayerController|SetbShowMouseCursor _returnvalue true)
  (EventDispatchers|BindEventtoSwitchon _returnvalue_2 (delegate Custom|LightOn)))

(event Custom|Increase%20Intensity
  (bind _returnvalue (Game|GetPlayerController 0))
  ;[1 1 1] Increase light cone
  (bind _returnvalue_2 (UserInterface|CreateWidget "/Game/UI/UI_David/WB_Welcome.WB_Welcome_C"))
  (UserInterface|Viewport|AddtoViewport _returnvalue_2 0)
  (Game|SetGamePaused true)
  (Input|SetInputModeUIOnly _returnvalue _returnvalue_2 "DoNotLock" false)
  (Variables|/Script/Engine.PlayerController|SetbShowMouseCursor _returnvalue true)
  (EventDispatchers|BindEventtoCorrectAnswer _returnvalue_2 (delegate Custom|IncreaseIntensity)))

(event Custom|LightOn
  ;[1 1 1] Switch on the light
  (Rendering|Components|Light|SetIntensity (Variables|Default|GetSpotLight) 3.5e+04)
  (Variables|/Script/Engine.PlayerController|SetbShowMouseCursor (Game|GetPlayerController 0) false))

(event Custom|IncreaseIntensity
  ;[1 1 1] Increase light cone
  (Rendering|Lighting|SetOuterConeAngle (Variables|Default|GetSpotLight) 1e+02)
  (Variables|/Script/Engine.PlayerController|SetbShowMouseCursor (Game|GetPlayerController 0) false))

(event EventBeginPlay)

(fn ConstructionScript)