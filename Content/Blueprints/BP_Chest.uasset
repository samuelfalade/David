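; BP_Chest is a chest that opens and lights up when an actor overlaps its Box, and closes when the overlap ends.
; BeginPlay creates dynamic materials for both halves, whose FadeAmount a reversed timeline drives on overlap.
; After the timeline and a delay, the lid is rotated and offset and the PointLight appears; exit hides the light, then resets fade and lid.
; The choice-widget and pause logic is disconnected.
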(event OnComponentBeginOverlap(Box)
  (params (OverlappedComponent :type Primitive%20Component%20Object%20Reference) (OtherActor :type Actor%20Object%20Reference) (OtherComp :type Primitive%20Component%20Object%20Reference) (OtherBodyIndex :type Integer) (bFromSweep :type Boolean) (SweepResult :type Hit%20Result%20Structure%20%28by%20ref%29))
  (bind _sm_chest_top (Variables|Default|GetSM_Chest_Top))
  ;[1 1 1] Open chest
  (Variables|Default|SetThirdPersonObject OtherActor)
  (bind _fadeamount (Timeline|OpenTimeline Reverse)
    (:Update
      (Rendering|Material|SetScalarParameterValue (Variables|Default|GetChestTopMat) "FadeAmount" _fadeamount :!class /Script/Engine.MaterialInstanceDynamic))
    (:Finished
      (Utilities|FlowControl|Delay 0.5)
      (Transformation|AddLocalRotation _sm_chest_top "35.000000,0.000000,0.000000" false false)
      (Transformation|AddLocalOffset _sm_chest_top "18.000000,0.000000,23.000000" false false)
      ;;[0 0.3419 0.09759] Turn Light on
      (Development|SetHiddeninGame (Variables|Default|GetPointLight) false false))))

(event OnComponentEndOverlap(Box)
  (params (OverlappedComponent :type Primitive%20Component%20Object%20Reference) (OtherActor :type Actor%20Object%20Reference) (OtherComp :type Primitive%20Component%20Object%20Reference) (OtherBodyIndex :type Integer))
  ;[1 1 1] Close chest
  (Variables|Default|SetThirdPersonObject OtherActor)
  ;;[0 0.3419 0.09759] Switch off light
  (Development|SetHiddeninGame (Variables|Default|GetPointLight) true false)
  (Utilities|FlowControl|Delay 0.5)
  (Rendering|Material|SetScalarParameterValue (Variables|Default|GetChestBottomMat) "FadeAmount" 1.0 :!class /Script/Engine.MaterialInstanceDynamic)
  (Transformation|ResetRelativeTransform (Variables|Default|GetSM_Chest_Top)))

(event EventBeginPlay
  (bind _returnvalue (Rendering|Material|CreateDynamicMaterialInstance (Variables|Default|GetSM_Chest_Bottom) 0 "/Game/Materials/M_Chest_Basic.M_Chest_Basic" "None" :!class /Script/Engine.PrimitiveComponent))
  (Variables|Default|SetChestBottomMat _returnvalue)
  (bind _returnvalue_2 (Rendering|Material|CreateDynamicMaterialInstance (Variables|Default|GetSM_Chest_Top) 0 "/Game/Materials/M_Chest_Basic.M_Chest_Basic" "None" :!class /Script/Engine.PrimitiveComponent))
  (Variables|Default|SetChestTopMat _returnvalue_2)
  (Rendering|Material|SetScalarParameterValue _returnvalue_2 "FadeAmount" 1.0 :!class /Script/Engine.MaterialInstanceDynamic))

(event Collision|EventActorBeginOverlap
  (params (OtherActor :type Actor%20Object%20Reference)))

(event EventTick
  (params (DeltaSeconds :type Float%20%28single-precision%29)))

(fn ConstructionScript)