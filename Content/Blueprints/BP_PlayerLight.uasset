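; Light actor that lets the player switch on a spotlight through a choice prompt when its trigger box is entered.
; The first overlap by any actor creates a WB_Choice widget, pauses the game and gives the UI input focus with the mouse cursor shown.
; The widget's SwitchOn dispatcher is bound to LightOn, which raises the spotlight intensity.
; Other custom events are empty, and some disconnected draft nodes remain.
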(event OnComponentBeginOverlap(Box)
  (params (OverlappedComponent :type Primitive%20Component%20Object%20Reference) (OtherActor :type Actor%20Object%20Reference) (OtherComp :type Primitive%20Component%20Object%20Reference) (OtherBodyIndex :type Integer) (bFromSweep :type Boolean) (SweepResult :type Hit%20Result%20Structure%20%28by%20ref%29))
  (bind _returnvalue (Game|GetPlayerController 0))
  (Variables|Default|SetThirdPersonObject OtherActor)
  (Utilities|FlowControl|DoOnce false
    (:Completed
      (bind _returnvalue_2 (UserInterface|CreateWidget "/Game/UI/WB_Choice.WB_Choice_C"))
      (UserInterface|Viewport|AddtoViewport _returnvalue_2 0)
      (Game|SetGamePaused true)
      (Input|SetInputModeUIOnly _returnvalue _returnvalue_2 "DoNotLock" false)
      (Variables|/Script/Engine.PlayerController|SetbShowMouseCursor _returnvalue true)
      (EventDispatchers|BindEventtoSwitchon _returnvalue_2 (delegate Custom|LightOn)))))

(event Custom|Custom%20intensity)

(event Custom|LightOn
  (Rendering|Components|Light|SetIntensity (Variables|Default|GetSpotLight) 1e+06)
  (Variables|/Script/Engine.PlayerController|SetbShowMouseCursor (Game|GetPlayerController 0) true))

(event EventBeginPlay
  ;[1 1 1] Starts light. UI starts on game start, not desired
)

(event EventTurnLighton
  (params (TurnLightOn :type Boolean)))

(fn ConstructionScript)