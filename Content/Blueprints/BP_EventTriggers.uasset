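; BP_EventTriggers is an actor with a Box trigger, apparently an unfinished event trigger tied to a pickup light.
; On BeginPlay it caches the player's third-person character, then casts its Light reference to BP_PickupLight and copies its own NewIntensity onto it.
; The Box overlap handler is empty, and disconnected nodes for capturing an overlapping pickup light once never run.
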(event OnComponentBeginOverlap(Box)
  (params (OverlappedComponent :type Primitive%20Component%20Object%20Reference) (OtherActor :type Actor%20Object%20Reference) (OtherComp :type Primitive%20Component%20Object%20Reference) (OtherBodyIndex :type Integer) (bFromSweep :type Boolean) (SweepResult :type Hit%20Result%20Structure%20%28by%20ref%29)))

(event EventBeginPlay
  (bind _asbp_third_person_character (Utilities|Casting|CastToBP_ThirdPersonCharacter (Game|GetPlayerCharacter 0)))
  (Variables|Default|SetAs%20BP%20Third%20Person%20Character _asbp_third_person_character)
  (bind _asbp_pickup_light (Utilities|Casting|CastToBP_PickupLight (Variables|Default|GetLight)))
  (Variables|/Game/Blueprints/BP_PickupLight.BP_PickupLight_C|SetNew%20Intensity _asbp_pickup_light (Variables|Default|GetNew%20Intensity)))

(event Collision|EventActorBeginOverlap
  (params (OtherActor :type Actor%20Object%20Reference)))

(event EventTick
  (params (DeltaSeconds :type Float%20%28single-precision%29)))

(fn ConstructionScript)