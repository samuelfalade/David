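; Replicated world pickup that a player collects with E, deducting its cost from the HUD account balance.
; ID selects a DT_Inventory row, unless DropItem overrides it, to set the label and blocking-load a skeletal mesh, falling back to static.
; Sphere overlap shows the prompt and enables input for the local player.
; A successful PickUpItemMessage on the character destroys the actor through DestroyServer and rewrites the balance text directly on WB_HUD.
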(event OnComponentBeginOverlap(Sphere)
  (params (OverlappedComponent :type Primitive%20Component%20Object%20Reference) (OtherActor :type Actor%20Object%20Reference) (OtherComp :type Primitive%20Component%20Object%20Reference) (OtherBodyIndex :type Integer) (bFromSweep :type Boolean) (SweepResult :type Hit%20Result%20Structure%20%28by%20ref%29))
  ;[1 1 1] set Interact UI visibility
  (bind _ascharacter (Utilities|Casting|CastToCharacter OtherActor))
  (bind _isnpc (Utilities|IsPlayer _ascharacter)
    (:true
      (Rendering|SetVisibility (Variables|Default|GetWidget) true false)
      (Input|EnableInput (Game|GetPlayerController 0))
      (Variables|Default|SetCharacter _ascharacter))
    (:false
      _))
  ;[1 1 1] Allow network access
  (if (not _isnpc)
    (Actor|SetOwner _ascharacter)))

(event OnComponentEndOverlap(Sphere)
  (params (OverlappedComponent :type Primitive%20Component%20Object%20Reference) (OtherActor :type Actor%20Object%20Reference) (OtherComp :type Primitive%20Component%20Object%20Reference) (OtherBodyIndex :type Integer))
  ;[1 1 1] set Interact UI visibility
  (bind _ascharacter (Utilities|Casting|CastToCharacter OtherActor))
  (Utilities|IsPlayer _ascharacter
    (:true
      (Rendering|SetVisibility (Variables|Default|GetWidget) false false)
      (Input|DisableInput (Game|GetPlayerController 0)))))

(event OnComponentBeginOverlap(Box)
  (params (OverlappedComponent :type Primitive%20Component%20Object%20Reference) (OtherActor :type Actor%20Object%20Reference) (OtherComp :type Primitive%20Component%20Object%20Reference) (OtherBodyIndex :type Integer) (bFromSweep :type Boolean) (SweepResult :type Hit%20Result%20Structure%20%28by%20ref%29))
  ;[1 1 1] Enable collectables
)

(event OnComponentEndOverlap(Box)
  (params (OverlappedComponent :type Primitive%20Component%20Object%20Reference) (OtherActor :type Actor%20Object%20Reference) (OtherComp :type Primitive%20Component%20Object%20Reference) (OtherBodyIndex :type Integer))
  ;[1 1 1] Enable collectables
)

(event Custom|Update
  (bind _item (Variables|Default|GetItem))
  (bind (_displayname _pickupmesh _pickupmeshstatic _cost) (Utilities|Struct|BreakST_Inventory_Item _item))
  ;[1 1 1] Load skeletal mesh
  (bind _aswb_pickup (Utilities|Casting|CastToWB_Pickup (UserInterface|GetWidget (Variables|Default|GetWidget))))
  (Rendering|Components|TextRender|SetText (Variables|/Game/Inventory/Widgets/WB_Pickup.WB_Pickup_C|GetTEXT _aswb_pickup) _displayname)
  (bind _returnvalue (Utilities|LoadAssetBlocking _pickupmesh))
  (bind _asskeletal_mesh (Utilities|Casting|CastToSkeletalMesh _returnvalue)
    (:then
      (Components|SkeletalMesh|SetSkeletalMeshAsset (Variables|Default|GetSkeletalMesh) _asskeletal_mesh)
      (Variables|Default|SetCost _cost))
    (:CastFailed
      ;[1 1 1] Load static mesh if skeletal mesh fails
      (bind _returnvalue_2 (Utilities|LoadAssetBlocking _pickupmeshstatic))
      (bind _asstatic_mesh (Utilities|Casting|CastToStaticMesh _returnvalue_2))
      (Components|StaticMesh|SetStaticMesh (Variables|Default|GetStaticMesh) _asstatic_mesh))))

(event Custom|Destroy%20server
  (Actor|DestroyActor))

(event Custom|Remove%20Cost)

(event EventBeginPlay
  (CallFunction|OnRepID))

(event Input|KeyboardEvents|E
  (params (Key :type Key%20Structure :default "None"))
  ;[1 1 1] Pick up items
  (:Pressed
    (bind _success (Class|BPIInventory|PickUpItem(Message) (Variables|Default|GetCharacter) (Variables|Default|GetID) (Variables|Default|GetItem) (Variables|Default|GetCost)))
    (if _success
      (bind _output_get (Variables|Default|SetCost (Variables|Default|GetCost)))
      (CallFunction|DestroyServer)
      ;[1 1 1] Update Acct Bal
      (bind _foundwidgets (Widget|GetAllWidgetsOfClass "/Game/UI/WB_HUD.WB_HUD_C" true))
      ;;[1 1 1] Print Acc bal, cost and the balance
      (Development|PrintString (Utilities|String|ToString(Float) (Math|Conversions|ToFloat(Integer) (Utilities|String|ToString(Text) (Variables|/Game/UI/WB_HUD.WB_HUD_C|GetAcct%20Bal (Utilities|Array|Get(acopy) _foundwidgets))))))
      (Development|PrintString (Utilities|String|ToString(Float) _output_get))
      (Development|PrintString (Utilities|String|ToString(Float) (- (Math|Conversions|ToFloat(Integer) (Utilities|String|ToString(Text) (Variables|/Game/UI/WB_HUD.WB_HUD_C|GetAcct%20Bal (Utilities|Array|Get(acopy) _foundwidgets)))) _output_get)))
      (Variables|/Game/UI/WB_HUD.WB_HUD_C|SetAcct%20Bal (Utilities|Array|Get(acopy) _foundwidgets) (Utilities|Text|ToText(String) (Utilities|String|ToString(Float) (- (Math|Conversions|ToFloat(Integer) (Utilities|String|ToString(Text) (Variables|/Game/UI/WB_HUD.WB_HUD_C|GetAcct%20Bal (Utilities|Array|Get(acopy) _foundwidgets)))) _output_get)))))))

(event Input|KeyboardEvents|R
  (params (Key :type Key%20Structure :default "None")))

(fn ConstructionScript
  (CallFunction|OnRepID))

(fn OnRepID
  (bind _returnvalue (Utilities|GetDataTableRow "/Game/Inventory/DT_Inventory.DT_Inventory" (Variables|Default|GetID))
    (:then
      (Variables|Default|SetItem (select (!= (Utilities|Struct|BreakST_Inventory_Item (Variables|Default|GetDropItem)) "") (Variables|Default|GetDropItem) _returnvalue))
      (CallFunction|Update))))

(fn OnRepCost)

(fn GetName
  (return (Variables|Default|GetName)))